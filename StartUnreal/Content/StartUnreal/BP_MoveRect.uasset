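; BP_MoveRect is an actor that moves its Cube component around a square path in its local X-Z plane.
; Each Tick, a MoveType state switch nudges the cube one unit Right, Up, Left or Down and advances to the next direction at that side's limit.
; The Right step lives in a MoveRight function that reports when the limit is passed.
; EventComponent's DoPlay and DoStop dispatchers toggle IsPlay to start and pause the motion.
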(event EventDispatcherDoPlay(EventComponent)
  (Variables|Default|SetIsPlay true))

(event EventDispatcherDoStop(EventComponent)
  (Variables|Default|SetIsPlay false))

(event EventTick
  (params (DeltaSeconds :type Float%20%28single-precision%29))
  (if (Variables|Default|GetIsPlay)
    (switch Utilities|FlowControl|Switch|SwitchonEN_MoveType (Variables|Default|GetMoveType)
      (:NewEnumerator0
        (bind _returnvalue (CallFunction|MoveRight))
        (if _returnvalue
          (Variables|Default|SetMoveType "NewEnumerator1")))
      (:NewEnumerator1
        (Transformation|AddRelativeLocation (Variables|Default|GetCube) "0.000000,0.000000,1.000000" false false)
        (if (> (.z (Variables|/Script/Engine.SceneComponent|GetRelativeLocation (Variables|Default|GetCube))) 1e+02)
          (Variables|Default|SetMoveType "NewEnumerator2")))
      (:NewEnumerator2
        (Transformation|AddRelativeLocation (Variables|Default|GetCube) "-1.000000,0.000000,0.000000" false false)
        (if (< (.x (Variables|/Script/Engine.SceneComponent|GetRelativeLocation (Variables|Default|GetCube))) 0.0)
          (Variables|Default|SetMoveType "NewEnumerator3")))
      (:NewEnumerator3
        (Transformation|AddRelativeLocation (Variables|Default|GetCube) "0.000000,0.000000,-1.000000" false false)
        (if (< (.z (Variables|/Script/Engine.SceneComponent|GetRelativeLocation (Variables|Default|GetCube))) 0.0)
          (Variables|Default|SetMoveType "NewEnumerator0"))))))

(fn ConstructionScript)

(fn MoveRight
  (Transformation|AddRelativeLocation (Variables|Default|GetCube) "1.000000,0.000000,0.000000" false false)
  (return (> (.x (Variables|/Script/Engine.SceneComponent|GetRelativeLocation (Variables|Default|GetCube))) 1e+02)))