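; BP_ActorSpawner is an actor that repeatedly spawns instances of the class held in its Class variable at its own transform.
; BeginPlay calls DoSpawnActor immediately, then sets a looping timer by function name to call it again every second.
; The spawner keeps no reference to spawned actors and sets no limit on their number.
; Disconnected rotation and interpolation nodes referring to Dragon and Player variables remain unused.
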(event EventBeginPlay
  (CallFunction|DoSpawnActor)
  (Utilities|Time|SetTimerbyFunctionName 0 "DoSpawnActor" 1.0 true))

(fn ConstructionScript)

(fn DoSpawnActor
  (Game|SpawnActorfromClass (Variables|Default|GetClass) (Transformation|GetActorTransform) "Undefined" "MultiplyWithRoot" 0 0))