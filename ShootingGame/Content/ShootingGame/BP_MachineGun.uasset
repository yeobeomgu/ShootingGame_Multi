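; BP_MachineGun is an automatic weapon for the shooting game that repeats its fire animation while the trigger is held.
; On press, EventTrigger calls LoopShootMontage at once and starts a looping timer on it by function name; on release it clears that timer.
; LoopShootMontage only plays the shoot montage from WeaponData on the owning character, with no projectile or damage logic in this Blueprint.
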(fn ConstructionScript
  (|CallParentFunction))

(fn EventTrigger
  (params (IsPress :type Boolean))
  (if IsPress
    (CallFunction|LoopShootMontage)
    (Utilities|Time|SetTimerbyFunctionName 0 "LoopShootMontage" 0.2 true)
    (else
      (Utilities|Time|ClearTimerbyFunctionName 0 "LoopShootMontage")))
  (return false))

(fn LoopShootMontage
  (Animation|PlayAnimMontage (Variables|Default|GetOwnChar) (.shootmontage (Variables|Default|GetWeaponData)) 1.0 "None"))