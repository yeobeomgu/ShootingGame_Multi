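; Player state for the shooting game that holds each player's health and magazine count.
; Health starts at max on BeginPlay, and damage and heal functions clamp it between zero and max; magazines can be added, or used only while above zero.
; RepNotify handlers on current HP and magazine count print debug messages and fire update event dispatchers so listeners can react to changes.
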(event EventBeginPlay
  (Variables|Default|SetCurHp (Variables|Default|GetMaxHp)))

(fn ConstructionScript)

(fn AddDamage
  (params (Damage :type Float%20%28double-precision%29))
  (Variables|Default|SetCurHp (Math|Float|Clamp(Float) (- (Variables|Default|GetCurHp) Damage) 0.0 (Variables|Default|GetMaxHp))))

(fn OnRepCurHp
  (Development|PrintString (Utilities|String|Append "OnRep_CurHp : " (Utilities|String|ToString(Float) (Variables|Default|GetCurHp))) true true "(R=0.000000,G=0.660000,B=1.000000,A=1.000000)" 6e+01)
  (Default|CallEventDispatcherUpdateMyHp (Variables|Default|GetCurHp) (Variables|Default|GetMaxHp)))

(fn AddMag
  (Variables|Default|SetMag (+ (Variables|Default|GetMag) 1)))

(fn OnRepMag
  (Development|PrintString (Utilities|String|Append "Mag : " (Utilities|String|ToString(Integer) (Variables|Default|GetMag))) true true "(R=0.000000,G=0.660000,B=1.000000,A=1.000000)" 6e+01)
  (Default|CallEventDispatcherUpdateMag (Variables|Default|GetMag)))

(fn UseMag
  (if (CallFunction|IsCanUseMag)
    (Variables|Default|SetMag (- (Variables|Default|GetMag) 1))
    (return true)
    (else
      (return false))))

(fn IsCanUseMag
  (return (> (Variables|Default|GetMag) 0)))

(fn AddHeal
  (params (Heal :type Float%20%28double-precision%29))
  (Variables|Default|SetCurHp (Math|Float|Clamp(Float) (+ (Variables|Default|GetCurHp) Heal) 0.0 (Variables|Default|GetMaxHp))))