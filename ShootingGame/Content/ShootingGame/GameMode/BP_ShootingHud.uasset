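; BP_ShootingHud is the shooting game's HUD, creating the ShootingHudWidget at BeginPlay and adding it to the viewport.
; It binds to the local BP_ShootingPlayerState's HP and magazine update dispatchers and seeds the initial HP display.
; If the player state is not ready, a short timer retries the binding.
; Setter functions forward HP, ammo and magazine values to the widget.
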(event EventBeginPlay
  (bind _returnvalue (UserInterface|CreateWidget "/Game/ShootingGame/Widget/ShootingHudWidget.ShootingHudWidget_C"))
  (bind _output_get (Variables|Default|SetHudWidget _returnvalue))
  (UserInterface|Viewport|AddtoViewport _output_get 0)
  (CallFunction|BindMyPlayerState))

(fn ConstructionScript)

(fn SetHudHp
  (params (CurHp :type Float%20%28double-precision%29) (MaxHp :type Float%20%28double-precision%29))
  (Default|SetHp (Variables|Default|GetHudWidget) CurHp MaxHp))

(fn BindMyPlayerState
  (bind _asbp_shooting_player_state (Utilities|Casting|CastToBP_ShootingPlayerState (Variables|/Script/Engine.Controller|GetPlayerState (Game|GetPlayerController 0)))
    (:then
      (EventDispatchers|BindEventtoEventDispatcherUpdateMyHp _asbp_shooting_player_state (EventDispatchers|CreateEvent :!event SetHudHp))
      (EventDispatchers|BindEventtoEventDispatcherUpdateMag _asbp_shooting_player_state (EventDispatchers|CreateEvent :!event SetHudMag))
      (CallFunction|SetHudHp (Variables|/Game/ShootingGame/GameMode/BP_ShootingPlayerState.BP_ShootingPlayerState_C|GetCurHp _asbp_shooting_player_state) (Variables|/Game/ShootingGame/GameMode/BP_ShootingPlayerState.BP_ShootingPlayerState_C|GetMaxHp _asbp_shooting_player_state)))
    (:CastFailed
      (Utilities|Time|SetTimerbyFunctionName 0 "BindMyPlayerState" 0.01))))

(fn SetHudAmmo
  (params (Ammo :type Byte))
  (Default|SetAmmo (Variables|Default|GetHudWidget) Ammo))

(fn SetHudMag
  (params (Mag :type Integer))
  (Default|SetMag (Variables|Default|GetHudWidget) Mag))